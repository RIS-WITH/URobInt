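; Interactive hinged door with a turnable handle, supporting both FPS key input and VR grabbing.
; In FPS, a trigger box enables input so E plays the handle timeline and toggles the door timeline.
; In VR, Tick uses atan2 on the grabbing controller's position to drive clamped handle and door angles.
; With a grabbable handle, the door swings only once turned or ajar; otherwise a Wrist grabbable drives it directly.
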(event `self.Box.OnComponentBeginOverlap`
  (params (OverlappedComponent :type "PrimitiveComponent Object Reference") (OtherActor :type "Actor Object Reference") (OtherComp :type "PrimitiveComponent Object Reference") (OtherBodyIndex :type Integer) (bFromSweep :type Boolean) (SweepResult :type "HitResult Structure (by ref)"))
  ;[1 1 1] FPS
  (`self.EnableInput` (`GameplayStatics.GetPlayerController` 0)))

(event `Key|E`
  (params (Key :type "Key Structure"))
  ;[1 1 1] FPS
  (:`Pressed`
    (`|ExecutionSequence`
      (:`then_0`
        (bind (_direction _handlerotation) (`Timeline|Timeline_1` :!via `PlayFromStart`)
          (:`Update`
            (`SceneComponent.K2_SetRelativeRotation` (`self.Handle`) (`KismetMathLibrary.MakeRotator` _handlerotation) false false))))
      (:`then_1`
        (if (`self.ClosedDoor`)
          (bind (_direction_2 _dooropen) (`Timeline|Timeline_0` :!label _label)
            (:`Update`
              (bind (_returnvalue_roll _returnvalue_pitch _returnvalue_yaw) (`KismetMathLibrary.BreakRotator` (`KismetMathLibrary.MakeRotator` 0.0 0.0 _dooropen)))
              (`SceneComponent.K2_SetRelativeRotation` (`self.door_right`) (`KismetMathLibrary.MakeRotator` 0.0 0.0 _returnvalue_yaw) false false)))
          (else
            (goto _label :!via `Reverse`)))))))

(event `self.Box.OnComponentEndOverlap`
  (params (OverlappedComponent :type "PrimitiveComponent Object Reference") (OtherActor :type "Actor Object Reference") (OtherComp :type "PrimitiveComponent Object Reference") (OtherBodyIndex :type Integer))
  ;[1 1 1] FPS
  (`self.DisableInput` (`GameplayStatics.GetPlayerController` 0)))

(event `self.ReceiveTick`
  (params (DeltaSeconds :type "Float (single-precision)"))
  ;[1 1 1] Vr
  (set `self.ClosedDoor` (< (stale `Key|E` _dooropen) 1.0))
  (`parent.ReceiveTick` DeltaSeconds)
  (bind _asbp_grapable (cast `/Game/VRTemplate/Blueprints/BP_grapable` (`ChildActorComponent.ChildActor` (`self.Handle`)))
    (:`then`
      (`self.rotation_handle` _asbp_grapable)
      (bind _movable_ (`self.Door Condition`))
      (if _movable_
        (`self.rotation_door` _asbp_grapable)))
    (:`CastFailed`
      (bind _asbp_grapable_2 (cast `/Game/VRTemplate/Blueprints/BP_grapable` (`ChildActorComponent.ChildActor` (`self.Wrist`))))
      (`self.rotation_door` _asbp_grapable_2))))

(event `self.ReceiveBeginPlay`
  ;[1 1 1] Vr
  (`parent.ReceiveBeginPlay`))

(fn `angle_min_max_door`
  (params (angle :type "Float (double-precision)"))
  (locals (angle_base :type "Float (single-precision)" :default 0.0))
  (bind _angle_door (`self.angle_door`))
  (bind _angle_door_2 (`self.angle_door`))
  (bind _angle_max_door (`self.angle_max_door`))
  (bind _angle_door_3 (`self.angle_door`))
  (bind (_returnvalue_roll _returnvalue_pitch _returnvalue_yaw) (`KismetMathLibrary.BreakRotator` (`SceneComponent.K2_GetComponentRotation` (`self.DoubleDoorFrame`))))
  (bind _returnvalue (* (- 360.0 (`self.angle_max_door`)) -1.0))
  (bind _output_get (set `local.angle_base` _returnvalue_yaw))
  (set `self.angle_door` (- angle _output_get))
  (if (< _angle_door_3 0.0)
    (if (< _angle_door_3 -360.0)
      (set `self.angle_door` (- _angle_door_3 -360.0)))
    (if (> _angle_door _returnvalue)
      (if (> (`KismetMathLibrary.Abs` (- _angle_door _returnvalue)) 50.0)
        (set `self.angle_door` (+ (`self.angle_min_door`) (`local.angle_base`)) :!label _label)
        (else
          (set `self.angle_door` (+ _angle_max_door (`local.angle_base`)) :!label _label_2)))
      (else
        (set `self.angle_door` (+ (`self.angle_door`) (`local.angle_base`)) :!label _label_3)))
    (elif (> _angle_door_2 _angle_max_door)
      (goto _label_2)
      (elif (> _angle_door_2 360.0)
        (goto _label)
        (else
          (goto _label_3))))))

(fn `angle_min_max_handle`
  (params (angle :type "Float (double-precision)"))
  (bind _angle_handle (`self.angle_handle`))
  (bind _returnvalue_roll (`KismetMathLibrary.BreakRotator` (`SceneComponent.K2_GetComponentRotation` (`self.Handle`))))
  (set `self.angle_handle` angle)
  (if (> (`KismetMathLibrary.Abs` (- (`self.angle_handle`) _returnvalue_roll)) 5.0)
    (set `self.angle_handle` _returnvalue_roll)
    (elif (< _angle_handle (`self.angle_min_handle`))
      (set `self.angle_handle` (`self.angle_min_handle`))
      (elif (> _angle_handle (`self.angle_max_handle`))
        (set `self.angle_handle` (`self.angle_max_handle`))))))

(fn `Door Condition`
  (returns (`movable?` :type Boolean))
  (bind (_returnvalue_roll _returnvalue_pitch _returnvalue_yaw) (`KismetMathLibrary.BreakRotator` (`SceneComponent.K2_GetComponentRotation` (`self.DoubleDoorFrame`))))
  (bind _returnvalue_roll_2 (`KismetMathLibrary.BreakRotator` (`SceneComponent.K2_GetComponentRotation` (`self.Handle`))))
  (bind (_returnvalue_roll_3 _returnvalue_pitch_2 _returnvalue_yaw_2) (`KismetMathLibrary.BreakRotator` (`SceneComponent.K2_GetComponentRotation` (`self.door_right`))))
  (return (or (> _returnvalue_roll_2 10.0) (!= _returnvalue_yaw_2 _returnvalue_yaw))))

(fn `rotation_door`
  (params (BP_Grapable :type "/Game/VRTemplate/Blueprints/BP_grapable Object Reference"))
  (bind _door_right (`self.door_right`))
  (bind (_returnvalue_roll _returnvalue_pitch _returnvalue_yaw) (`KismetMathLibrary.BreakRotator` (`SceneComponent.K2_GetComponentRotation` _door_right)))
  (bind (_returnvalue_x _returnvalue_y) (`KismetMathLibrary.BreakVector` (- (`SceneComponent.K2_GetComponentLocation` (`/Game/VRTemplate/Blueprints/BP_grapable.motionControlerRef` BP_Grapable)) (`SceneComponent.K2_GetComponentLocation` (`self.door_right`)))))
  (bind _returnvalue (+ (`KismetMathLibrary.DegAtan2` _returnvalue_y _returnvalue_x) 90.0))
  (if (`/Game/VRTemplate/Blueprints/BP_grapable.bIsHeld` BP_Grapable)
    (if (not (!= (`self.distance_hand_handle`) 0.0))
      (set `self.distance_hand_handle` (- _returnvalue _returnvalue_yaw)))
    (`self.angle_min_max_door` (- _returnvalue (`self.distance_hand_handle`)))
    (`SceneComponent.K2_SetWorldRotation` _door_right (`KismetMathLibrary.MakeRotator` _returnvalue_roll _returnvalue_pitch (`self.angle_door`)) false false)
    (else
      (set `self.distance_hand_handle` 0.0))))

(fn `rotation_handle`
  (params (BP_Grapable :type "/Game/VRTemplate/Blueprints/BP_grapable Object Reference"))
  (bind _returnvalue (`SceneComponent.K2_GetComponentToWorld` (`self.door_right`)))
  (bind (_returnvalue_roll _returnvalue_pitch _returnvalue_yaw) (`KismetMathLibrary.BreakRotator` (`SceneComponent.K2_GetComponentRotation` (`self.Handle`))))
  (bind (_returnvalue_roll_2 _returnvalue_pitch_2 _returnvalue_yaw_2) (`KismetMathLibrary.BreakRotator` (`SceneComponent.K2_GetComponentRotation` (`self.Handle`))))
  (bind (_returnvalue_x _returnvalue_y _returnvalue_z) (`KismetMathLibrary.BreakVector` (- (`KismetMathLibrary.InverseTransformLocation` _returnvalue (`SceneComponent.K2_GetComponentLocation` (`/Game/VRTemplate/Blueprints/BP_grapable.motionControlerRef` BP_Grapable))) (`KismetMathLibrary.InverseTransformLocation` _returnvalue (`SceneComponent.K2_GetComponentLocation` (`self.Handle`))))))
  (if (`/Game/VRTemplate/Blueprints/BP_grapable.bIsHeld` BP_Grapable)
    (`self.angle_min_max_handle` (+ (`KismetMathLibrary.DegAtan2` _returnvalue_y _returnvalue_z) -90.0))
    (`SceneComponent.K2_SetWorldRotation` (`self.Handle`) (`KismetMathLibrary.MakeRotator` (`self.angle_handle`) _returnvalue_pitch _returnvalue_yaw) false false)
    (elif (> _returnvalue_roll_2 0.0)
      (`SceneComponent.K2_SetWorldRotation` (`self.Handle`) (`KismetMathLibrary.MakeRotator` (- _returnvalue_roll_2 2.0) _returnvalue_pitch_2 _returnvalue_yaw_2) false false))))

(fn `UserConstructionScript`)