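; Two-floor elevator actor: overlapping the interior or either floor's trigger box enables player input, letting NumPad One and Zero send the car up or down.
; A timeline lerps the Interior between Start and End, with CanControl blocking new calls until it finishes.
; Separate timelines open the top or bottom four-piece door set after a fixed delay, then reverse to close it, independent of the car's actual arrival.
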(event `self.interior hit box.OnComponentBeginOverlap`
  (params (OverlappedComponent :type "PrimitiveComponent Object Reference") (OtherActor :type "Actor Object Reference") (OtherComp :type "PrimitiveComponent Object Reference") (OtherBodyIndex :type Integer) (bFromSweep :type Boolean) (SweepResult :type "HitResult Structure (by ref)"))
  (`self.EnableInput` (`GameplayStatics.GetPlayerController` 0)))

(event `self.interior hit box.OnComponentEndOverlap`
  (params (OverlappedComponent :type "PrimitiveComponent Object Reference") (OtherActor :type "Actor Object Reference") (OtherComp :type "PrimitiveComponent Object Reference") (OtherBodyIndex :type Integer))
  (`self.DisableInput` (`GameplayStatics.GetPlayerController` 0)))

(event `self.0eme.OnComponentBeginOverlap`
  (params (OverlappedComponent :type "PrimitiveComponent Object Reference") (OtherActor :type "Actor Object Reference") (OtherComp :type "PrimitiveComponent Object Reference") (OtherBodyIndex :type Integer) (bFromSweep :type Boolean) (SweepResult :type "HitResult Structure (by ref)"))
  (`self.EnableInput` (`GameplayStatics.GetPlayerController` 0)))

(event `Key|NumPadOne`
  (params (Key :type "Key Structure"))
  (:`Pressed`
    (if (`self.can_control`)
      (set `self.can_control` false)
      (`|ExecutionSequence`
        (:`then_0`
          ;[1 1 1] elevator
          (bind (_direction _newtrack_0) (`Timeline|Timeline_0` :!label _label)
            (:`Update`
              (`SceneComponent.K2_SetRelativeLocation` (`self.interior`) (`KismetMathLibrary.VLerp` (`self.Start`) (`self.End`) _newtrack_0) false false))
            (:`Finished`
              (set `self.can_control` true))))
        (:`then_1`
          ;[1 1 1] up door
          (`KismetSystemLibrary.Delay` 3.0) ; OPEN
          (bind (_direction_2 _newtrack_0_2) (`Timeline|Timeline_2` :!label _label_2)
            (:`Update`
              (`|ExecutionSequence`
                (:`then_0`
                  (`SceneComponent.K2_SetRelativeTransform` (`self.top door half 1`) (`KismetMathLibrary.TLerp` (`self.A_1`) (`self.B_0`) _newtrack_0_2) false false))
                (:`then_1`
                  (`SceneComponent.K2_SetRelativeTransform` (`self.top door half`) (`KismetMathLibrary.TLerp` (`self.A_20`) (`self.B_10`) _newtrack_0_2) false false))
                (:`then_2`
                  (`SceneComponent.K2_SetRelativeTransform` (`self.door top in 1`) (`KismetMathLibrary.TLerp` (`self.A_4`) (`self.B_3`) _newtrack_0_2) false false))
                (:`then_3`
                  (`SceneComponent.K2_SetRelativeTransform` (`self.door top in`) (`KismetMathLibrary.TLerp` (`self.A_5`) (`self.B_4`) _newtrack_0_2) false false))))))
        (:`then_2`
          (`KismetSystemLibrary.Delay` 5.0) ; CLOSE
          (goto _label_2 :!via `Reverse`))))))

(event `self.0eme.OnComponentEndOverlap`
  (params (OverlappedComponent :type "PrimitiveComponent Object Reference") (OtherActor :type "Actor Object Reference") (OtherComp :type "PrimitiveComponent Object Reference") (OtherBodyIndex :type Integer))
  (`self.DisableInput` (`GameplayStatics.GetPlayerController` 0)))

(event `Key|NumPadZero`
  (params (Key :type "Key Structure"))
  (:`Pressed`
    (if (`self.can_control`)
      (set `self.can_control` false)
      (`|ExecutionSequence`
        (:`then_0`
          (goto _label :!via `Reverse`))
        (:`then_1`
          ;[1 1 1] door down
          (`KismetSystemLibrary.Delay` 3.0) ; OPEN
          (bind (_direction _newtrack_0) (`Timeline|Timeline_1` :!label _label_3)
            (:`Update`
              (`|ExecutionSequence`
                (:`then_0`
                  (`SceneComponent.K2_SetRelativeTransform` (`self.botom door half`) (`KismetMathLibrary.TLerp` (`self.A_8`) (`self.B_6`) _newtrack_0) false false))
                (:`then_1`
                  (`SceneComponent.K2_SetRelativeTransform` (`self.botom door half 1`) (`KismetMathLibrary.TLerp` (`self.A_7`) (`self.B_5`) _newtrack_0) false false))
                (:`then_2`
                  (`SceneComponent.K2_SetRelativeTransform` (`self.door bot in 1`) (`KismetMathLibrary.TLerp` (`self.A_6`) (`self.B_1`) _newtrack_0) false false))
                (:`then_3`
                  (`SceneComponent.K2_SetRelativeTransform` (`self.door bot in`) (`KismetMathLibrary.TLerp` (`self.A_6`) (`self.B_2`) _newtrack_0) false false))))))
        (:`then_2`
          (`KismetSystemLibrary.Delay` 5.0) ; CLOSE
          (goto _label_3 :!via `Reverse`))))))

(event `self.1eme.OnComponentBeginOverlap`
  (params (OverlappedComponent :type "PrimitiveComponent Object Reference") (OtherActor :type "Actor Object Reference") (OtherComp :type "PrimitiveComponent Object Reference") (OtherBodyIndex :type Integer) (bFromSweep :type Boolean) (SweepResult :type "HitResult Structure (by ref)"))
  (`self.EnableInput` (`GameplayStatics.GetPlayerController` 0)))

(event `self.1eme.OnComponentEndOverlap`
  (params (OverlappedComponent :type "PrimitiveComponent Object Reference") (OtherActor :type "Actor Object Reference") (OtherComp :type "PrimitiveComponent Object Reference") (OtherBodyIndex :type Integer))
  (`self.DisableInput` (`GameplayStatics.GetPlayerController` 0)))

(fn `UserConstructionScript`)